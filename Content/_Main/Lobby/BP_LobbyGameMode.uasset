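; Lobby game mode that tracks connected players, host-selected map settings, character choices and kicks for a multiplayer session.
; PostLogin registers each controller and passes it server and map info, while UpdateEveryone and host setting changes push updates to all clients through interface messages.
; ChangeCharacter spawns and possesses the chosen pawn at the last PlayerStart found.
; Starting shows loading screens on every client, then servertravels to the level matching the map ID.
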(event Custom|SpawnPlayer
  (params (Player :type Player%20Controller%20Object%20Reference)))

(event Custom|StartLoadingScreen
  ;[1 1 1] Load the game
  (for _array_element (Variables|Default|GetConnectedPlayers)
    (bind _lobbypc (Class|BPILobbyPC|LobbyPcRef(Message) _array_element))
    (Default|ShowLoadingScreen _lobbypc))
  (CallFunction|LaunchGame))

(event Custom|HostUpdateGameSettings
  (params (SelectedMapImage :type Texture%202D%20Object%20Reference) (SelectedMapName :type String) (SelectedMapTime :type String) (SelectedMapID :type Integer))
  ;[1 1 1] Update lobby for each client when smth changes on server
  (Variables|Default|SetSelectedMapImage SelectedMapImage)
  (Variables|Default|SetSelectedMapName SelectedMapName)
  (Variables|Default|SetSelectedMapTime SelectedMapTime)
  (Variables|Default|SetSelectedMapID SelectedMapID)
  (for _array_element (Variables|Default|GetConnectedPlayers)
    (bind _lobbypc (Class|BPILobbyPC|LobbyPcRef(Message) _array_element))
    (Default|UpdateLobbySettings _lobbypc (Variables|Default|GetSelectedMapImage) (Variables|Default|GetSelectedMapName) (Variables|Default|GetSelectedMapTime))))

(event Custom|PlayerKicked
  (params (PlayerID :type Integer))
  ;[1 1 1] Kick selected player from game session / lobby
  (bind _lobbypc (Class|BPILobbyPC|LobbyPcRef(Message) (Utilities|Array|Get(acopy) (Variables|Default|GetConnectedPlayers) PlayerID)))
  (Default|Kicked _lobbypc))

(event Custom|UpdateEveryone
  (bind _connectedplayers (Variables|Default|GetConnectedPlayers))
  ;[1 1 1] Update all connected players lobby widget info
  (bind _output_get (Variables|Default|SetCurrentPlayersCount (Utilities|Array|Length (Variables|Default|GetConnectedPlayers))))
  (if (> _output_get 0)
    (Utilities|Array|Clear (Variables|Default|GetConnectedPlayersInfo))
    (for _array_element _connectedplayers
      (bind _lobbypc (Class|BPILobbyPC|LobbyPcRef(Message) _array_element))
      (Utilities|Array|AddUnique (Variables|Default|GetConnectedPlayersInfo) (Variables|/Game/_Main/Lobby/BP_LobbyPC.BP_LobbyPC_C|GetPlayerSettings _lobbypc))
      (Default|UpdatePlayersCount _lobbypc (Variables|Default|GetCurrentPlayersCount) (Variables|Default|GetMaxPlayers)))
    (for _array_element_2 _connectedplayers
      (bind _lobbypc_2 (Class|BPILobbyPC|LobbyPcRef(Message) _array_element_2))
      (Default|AddPlayerInfo _lobbypc_2 (Variables|Default|GetConnectedPlayersInfo))
      (CallFunction|AddtoKickList))
    (bind _array_element_3 (Utilities|Array|ForEachLoopwithBreak (Variables|Default|GetConnectedPlayersInfo))
      (:LoopBody
        (if (== (.PlayerCharacter (Utilities|Struct|BreakS_PlayerInfo _array_element_3)) 0)
          (Variables|Default|SetCanStart false)
          (CallFunction|CannotStartGame)
          (else
            (Variables|Default|SetCanStart true)))))))

(event Custom|AddToKickList
  ;[1 1 1] Add connected players tp kick list
  ;;[1 1 1] Host is at index 0 so only host will see this window
  (bind _lobbypc (Class|BPILobbyPC|LobbyPcRef(Message) (Game|GetPlayerController 0)))
  (Default|AddPlayertoKickWindow _lobbypc))

(event Custom|CannotStartGame
  ;[1 1 1] Update all connected players lobby widget info
  (Utilities|Array|ForEachLoopwithBreak (Variables|Default|GetConnectedPlayersInfo)) ; enters at Break
)

(event Custom|LaunchGame
  (bind _returnvalue (Game|GetPlayerController 0))
  ;[1 1 1] Load the game
  (switch int (Variables|Default|GetSelectedMapID)
    (:0
      (Development|ExecuteConsoleCommand "servertravel /Game/Maps/Level01" _returnvalue))
    (:1
      (Development|ExecuteConsoleCommand "servertravel /Game/Maps/Level02" _returnvalue))))

(event Custom|ChangeCharacter
  (params (ConnectedPlayer :type Player%20Controller%20Object%20Reference) (CharacterClass :type Character%20Class%20Reference) (StatusChanged :type Boolean))
  (bind _spawnpoints (Variables|Default|GetSpawnPoints))
  ;[1 1 1] Spawn Player character
  (if (not StatusChanged)
    (Utilities|IsValid (Pawn|GetControlledPawn ConnectedPlayer)
      (:Is%20Valid
        (Actor|DestroyActor))
      (:Is%20Not%20Valid
        _))
    (bind _returnvalue (Game|SpawnActorfromClass CharacterClass (Transformation|GetActorTransform (Utilities|Array|Get(acopy) _spawnpoints (- (Utilities|Array|Length _spawnpoints) 1))) "AlwaysSpawn" 0 0))
    (Pawn|Possess ConnectedPlayer _returnvalue)))

(event EventOnLogout
  (params (ExitingController :type Controller%20Object%20Reference))
  ;[1 1 1] Remove the connected player infom then update everyone with new info
  (bind (_array_element _array_index) (Utilities|Array|ForEachLoopwithBreak (Variables|Default|GetConnectedPlayers) :!label _label)
    (:LoopBody
      (if (== _array_element ExitingController)
        (goto _label Break)))
    (:Completed
      (Utilities|Array|RemoveIndex (Variables|Default|GetConnectedPlayers) _array_index)
      (Utilities|Array|RemoveIndex (Variables|Default|GetConnectedPlayersInfo) _array_index)
      (CallFunction|UpdateEveryone))))

(event EventPostLogin
  (params (NewPlayer :type Player%20Controller%20Object%20Reference))
  ;[1 1 1] Initial setup, runs each time player connects to session, lobby updates for each connected client
  (bind _output_get (Variables|Default|SetConnectedPlayer NewPlayer))
  (Utilities|Array|AddUnique (Variables|Default|GetConnectedPlayers) _output_get)
  (bind _outactors (Actor|GetAllActorsOfClass "/Script/Engine.PlayerStart"))
  (Variables|Default|SetSpawnPoints _outactors)
  (bind _gameinstance (Class|BPIGameInstance|MainGameInstanceRef(Message) (Game|GetGameInstance)))
  (Variables|Default|SetServerName (Variables|/Game/_Main/MainGameInstance.MainGameInstance_C|GetServerName _gameinstance))
  (Variables|Default|SetMaxPlayers (Variables|/Game/_Main/MainGameInstance.MainGameInstance_C|GetMaxPlayers _gameinstance))
  (bind _lobbypc (Class|BPILobbyPC|LobbyPcRef(Message) (Variables|Default|GetConnectedPlayer)))
  (bind _output_get_2 (Variables|Default|SetLobbyPC _lobbypc))
  (Default|InitialSetup _output_get_2 (Variables|Default|GetServerName) (Variables|Default|GetSelectedMapImage) (Variables|Default|GetSelectedMapName) (Variables|Default|GetSelectedMapTime)))

(fn ConstructionScript)

(fn LobbyGameModeRef
  (return self))